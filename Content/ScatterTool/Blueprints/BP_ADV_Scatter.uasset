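; Editor-placed scatter tool that fills a box area with randomly placed instanced meshes at construction time.
; The construction script sizes the preview box, creates one instanced mesh component per mesh type, then draws seeded random points with optional centre clustering.
; A sphere trace above each point rejects blocked spots, retrying through a DoN limit.
; Clear spots get a random mesh, yaw and scale, with optional shrinking toward the edges.
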(fn `UserConstructionScript`
  (bind _radius (`self.Radius`))
  (bind _radius_2 (`self.Radius`))
  (bind _instanced_meshes (`self.Instanced Meshes`))
  (bind _meshes_to_spawn (`self.Meshes to spawn`))
  (bind _radius_3 (`self.Radius`))
  (bind _random_seed (`self.Random Seed`))
  (bind _collision_trace_range (`self.Collision Trace Range`))
  (bind _returnvalue (/ _collision_trace_range 5.0))
  (bind _returnvalue_2 (* _radius_3 -1.0))
  (bind _returnvalue_3 (+ (`self.K2_GetActorLocation`) (`self.Spawn Point`)))
  (bind _returnvalue_4 (`KismetMathLibrary.RandomFloatInRangeFromStream` 1.0 (`KismetMathLibrary.SelectFloat` 1.8 1.0 (`self.Cluster Around Centre`)) _random_seed))
  (bind _returnvalue_5 (* (`KismetMathLibrary.SelectFloat` (`KismetMathLibrary.FClamp` (/ (- (/ _radius_2 0.7) (`KismetMathLibrary.VSize` (`self.Spawn Point`))) _radius_2) 0.6) 1.0 (`self.Scale Falloff`)) (`KismetMathLibrary.RandomFloatInRangeFromStream` (`self.Scale Min`) (`self.Scale Max`) (`self.Random Seed`))))
  ;[1 1 1] Spawn Area Size Control
  (`BoxComponent.SetBoxExtent` (`self.Radius_Vis`) (`KismetMathLibrary.MakeVector` _radius _radius (`self.Collision Trace Range`)) true)
  ;[1 1 1] Create instanced static mesh to use as templates, once for each mesh type
  (for _index (range (+ (`KismetArrayLibrary.Array_Length` _meshes_to_spawn) 1))
    (bind _returnvalue_6 (`AddComponent|NODE_AddInstancedStaticMeshComponent-0`))
    (`StaticMeshComponent.SetStaticMesh` _returnvalue_6 (`|GetArrayItem` _meshes_to_spawn _index))
    (`KismetArrayLibrary.Array_Add` (`self.Instanced Meshes`) _returnvalue_6))
  (for _ (range 1 (+ (`KismetMathLibrary.Clamp` (`self.Number of meshes`) 1 10000) 1))
    (set `self.Spawn Point` (`KismetMathLibrary.MakeVector` (/ (`KismetMathLibrary.RandomFloatInRangeFromStream` _returnvalue_2 _radius_3 _random_seed) _returnvalue_4) (/ (`KismetMathLibrary.RandomFloatInRangeFromStream` _returnvalue_2 _radius_3 _random_seed) _returnvalue_4) (`KismetMathLibrary.RandomFloatInRangeFromStream` -15.0 -4.0 _random_seed)) :!label _label)
    ;[1 1 1] Comment
    (bind (_outhit _returnvalue_7) (`KismetSystemLibrary.SphereTraceSingle` (+ (`KismetMathLibrary.MakeVector` 0.0 0.0 _collision_trace_range) _returnvalue_3) (+ (`KismetMathLibrary.MakeVector` 0.0 0.0 (/ _returnvalue 1.0)) _returnvalue_3) _returnvalue "TraceTypeQuery1" true))
    (if _returnvalue_7
      (`/Engine/EditorBlueprintResources/StandardMacros.Do N` 0 :!label _label_2
        (:`Exit`
          (goto _label)))
      (else
        (`|ExecutionSequence`
          (:`then_0`
            (goto _label_2 :!via `Reset`))
          (:`then_1`
            (`InstancedStaticMeshComponent.AddInstance` (`|GetArrayItem` _instanced_meshes (`KismetMathLibrary.RandomIntegerInRangeFromStream` 0 (`KismetArrayLibrary.Array_Length` _instanced_meshes) (`self.Random Seed`))) (`KismetMathLibrary.MakeTransform` (- (`self.Spawn Point`) (0.0 0.0 -10.0)) (`KismetMathLibrary.MakeRotator` 0.0 0.0 (`KismetMathLibrary.RandomFloatInRangeFromStream` 0.0 360.0 (`self.Random Seed`))) (`KismetMathLibrary.MakeVector` _returnvalue_5 _returnvalue_5 _returnvalue_5)))))))))